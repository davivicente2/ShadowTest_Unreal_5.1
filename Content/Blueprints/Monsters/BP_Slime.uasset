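; Flipbook-sprite slime enemy that patrols along the X axis, attacks the player and can be killed.
; Tick drives animation and movement, with a forward visibility trace that pauses the slime, then reverses it.
; HitBox overlaps with BP_Slime actors (not the player) start a delayed attack that damages the player via a pawn trace, then cools down.
; Damage knocks it away from the causer; at zero health it plays dust and is destroyed.
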(event OnComponentBeginOverlap(HitBox)
  (params (OverlappedComponent :type Primitive%20Component%20Object%20Reference) (OtherActor :type Actor%20Object%20Reference) (OtherComp :type Primitive%20Component%20Object%20Reference) (OtherBodyIndex :type Integer) (bFromSweep :type Boolean) (SweepResult :type Hit%20Result%20Structure%20%28by%20ref%29))
  (Utilities|Casting|CastToBP_Slime OtherActor)
  (bind _returnvalue (Utilities|Time|SetTimerbyEvent (delegate Custom|AtackPlayer) 1.0))
  (Variables|Default|SetAtackEvent _returnvalue))

(event OnComponentEndOverlap(HitBox)
  (params (OverlappedComponent :type Primitive%20Component%20Object%20Reference) (OtherActor :type Actor%20Object%20Reference) (OtherComp :type Primitive%20Component%20Object%20Reference) (OtherBodyIndex :type Integer))
  (bind _returnvalue (Transformation|GetActorLocation))
  (Utilities|Casting|CastToBP_Slime OtherActor)
  (Utilities|Time|ClearandInvalidateTimerbyHandle (Variables|Default|GetAtackEvent))
  (Utilities|FlowControl|DoOnce false) ; enters at Reset
)

(event Custom|AnimationUpdate
  (bind _slime_idle (Variables|Default|GetSlime_Idle))
  (Sprite|SetFlipbook (Variables|Default|GetSprite) (select (> (Math|Vector|VectorLength (Variables|/Script/Engine.MovementComponent|GetVelocity (Variables|Character|GetCharacterMovement))) 0.0) _slime_idle _slime_idle)))

(event Custom|MovimentUpdate
  (bind _returnvalue (Transformation|GetActorLocation))
  (Utilities|FlowControl|Sequence
    (:then_0
      (if (> (Variables|Default|GetMoviment%20Direction) 0.0)
        (Transformation|SetActorRotation "0, 0, 0")
        (else
          (Transformation|SetActorRotation "0.000000,180.000000,0.000000"))))
    (:then_1
      (Pawn|Input|AddMovementInput "1.000000,0.000000,0.000000" (Variables|Default|GetMoviment%20Direction) false)
      (bind _returnvalue_2 (Collision|LineTraceByChannel _returnvalue (+ _returnvalue (* (Transformation|GetActorForwardVector) (Math|Vector|MakeVector 3e+02 0.0 0.0))) "TraceTypeQuery1" false 0 "None"))
      (if _returnvalue_2
        (Utilities|FlowControl|DoOnce false :!label _label
          (:Completed
            (Variables|/Script/Engine.CharacterMovementComponent|SetMaxWalkSpeed (Variables|Character|GetCharacterMovement) 0.0)
            (Utilities|FlowControl|Delay (Variables|Default|GetDuration))
            (Variables|/Script/Engine.CharacterMovementComponent|SetMaxWalkSpeed (Variables|Character|GetCharacterMovement) (Variables|Default|GetMax%20Walk%20Speed))
            (Variables|Default|SetMoviment%20Direction (* (Variables|Default|GetMoviment%20Direction) -1.0))
            (goto _label Reset)))))))

(event Custom|AtackPlayer
  (bind _returnvalue (Transformation|GetActorLocation))
  (if (not (Variables|Default|GetIs%20Enemy%20Dead?))
    (Utilities|FlowControl|DoOnce false :!label _label
      (:Completed
        (Variables|Default|SetIs%20Enemy%20Attacking? true)
        (Utilities|FlowControl|Delay (Class|PaperFlipbook|GetTotalDuration (Variables|Default|GetSlime_Idle)))
        (Utilities|FlowControl|Sequence
          (:then_0
            (Variables|Default|SetIs%20Enemy%20Attacking? false))
          (:then_1
            (bind _outhit (Collision|LineTraceForObjects _returnvalue (+ _returnvalue (* (Transformation|GetActorForwardVector) (Math|Vector|MakeVector 1e+02 0.0 0.0))) (Utilities|Array|MakeArray "ObjectTypeQuery3") false (Utilities|Array|MakeArray self) "None"))
            (if (== (Game|GetPlayerCharacter 0) (.HitActor (Collision|BreakHitResult _outhit)))
              (Game|Damage|ApplyDamage (.HitActor (Collision|BreakHitResult _outhit)) (Variables|Default|GetBase%20Damage) 0 self))
            (Utilities|FlowControl|Delay (Variables|Default|GetAtackCooldown))
            (goto _label Reset)))))))

(event Game|Damage|EventAnyDamage
  (params (Damage :type Float%20%28single-precision%29) (DamageType :type Damage%20Type%20Object%20Reference) (InstigatedBy :type Controller%20Object%20Reference) (DamageCauser :type Actor%20Object%20Reference))
  (Variables|Default|SetEnemyHelath (- (Variables|Default|GetEnemyHelath) Damage))
  (Character|LaunchCharacter (Math|Vector|MakeVector (* (select (< (.x (Math|Vector|Normalize (Math|Vector|GetUnitDirection(Vector) (Transformation|GetActorLocation DamageCauser) (Transformation|GetActorLocation)))) 0.0) 1.0 -1.0) -1.5e+02) 0.0 0.0) true true)
  (if (<= (Variables|Default|GetEnemyHelath) 0.0)
    (Variables|Default|SetIs%20Enemy%20Dead? true)
    (Sprite|SetFlipbook (Variables|Default|GetSprite) "/Game/Assets/Flipbooks/Efects/FB_DustFall.FB_DustFall")
    (Utilities|FlowControl|Delay 0.1)
    (Sprite|SetFlipbook (Variables|Default|GetSprite))
    (Utilities|FlowControl|Delay 1.0)
    (Actor|DestroyActor)
    (else
      (Variables|Default|SetIs%20Enemy%20Dead? false))))

(event EventTick
  (params (DeltaSeconds :type Float%20%28single-precision%29))
  (if (not (Variables|Default|GetIs%20Enemy%20Dead?))
    (if (Variables|Default|GetIs%20Enemy%20Attacking?)
      (Sprite|SetFlipbook (Variables|Default|GetSprite) "/Game/Assets/Flipbooks/Monsters/FB_SlimeTest.FB_SlimeTest")
      (Utilities|FlowControl|Delay 2.0)
      (Variables|Default|SetIs%20Enemy%20Attacking? false)
      (else
        (CallFunction|AnimationUpdate)
        (CallFunction|MovimentUpdate)))))

(event EventBeginPlay
  (Variables|/Script/Engine.CharacterMovementComponent|SetMaxWalkSpeed (Variables|Character|GetCharacterMovement) (Variables|Default|GetMax%20Walk%20Speed)))

(fn ConstructionScript)