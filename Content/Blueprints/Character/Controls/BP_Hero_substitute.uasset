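; BP_Hero_substitute is a side-scrolling sprite hero character handling jump, attack and horizontal movement input.
; Jump, ledge, landing and attack events drive animation node jumps, while Tick turns the controller left or right from X velocity.
; Landing stops movement and sets IsMovimentLocked, but movement and facing never check that flag.
; Damage only prints a debug message, and SpawnDust spawns landing dust at the sprite without being called here.
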(event EventOnJumped
  (Class|PaperZDAnimInstance|JumptoNode (Variables|/Script/PaperZD.PaperZDAnimationComponent|GetAnimInstance (Variables|Default|GetAnimationComponent)) "AirBorne" "None"))

(event EventOnWalkingOffLedge
  (params (PreviousFloorImpactNormal :type Vector%20%28by%20ref%29 :default "0, 0, 0") (PreviousFloorContactNormal :type Vector%20%28by%20ref%29 :default "0, 0, 0") (PreviousLocation :type Vector%20%28by%20ref%29 :default "0, 0, 0") (TimeDelta :type Float%20%28single-precision%29))
  (Class|PaperZDAnimInstance|JumptoNode (Variables|/Script/PaperZD.PaperZDAnimationComponent|GetAnimInstance (Variables|Default|GetAnimationComponent)) "AirBorne" "None"))

(event EventTick
  (params (DeltaSeconds :type Float%20%28single-precision%29))
  (bind _returnvalue (Pawn|GetController))
  (bind _returnvalue_2 (Pawn|GetController))
  (|CallParentFunction DeltaSeconds)
  (if true ; If we can't move, force updating to last direction
    (Math|Float|CompareFloat (.X (Math|Vector|BreakVector (Variables|/Script/Engine.MovementComponent|GetVelocity (Pawn|GetMovementComponent)))) 0.0
      (:>
        ;[0 0.4745 1] Look Right
        (Utilities|IsValid _returnvalue_2
          (:Is%20Valid
            (Pawn|SetControlRotation _returnvalue_2 (Math|Rotator|MakeRotator 0.0 0.0 0.0)))))
      (:<
        ;[0 0.4745 1] Look Left
        (Utilities|IsValid _returnvalue
          (:Is%20Valid
            (Pawn|SetControlRotation _returnvalue (Math|Rotator|MakeRotator 0.0 0.0 1.8e+02))))))))

(event EventOnLanded
  (params (Hit :type Hit%20Result%20Structure%20%28by%20ref%29))
  (Class|PaperZDAnimInstance|JumptoNode (Variables|/Script/PaperZD.PaperZDAnimationComponent|GetAnimInstance (Variables|Default|GetAnimationComponent)) "Landed" "None")
  (Components|Movement|StopMovementImmediately (Variables|Character|GetCharacterMovement))
  (Variables|Default|SetIsMovimentLocked true))

(event Game|Damage|EventAnyDamage
  (params (Damage :type Float%20%28single-precision%29) (DamageType :type Damage%20Type%20Object%20Reference) (InstigatedBy :type Controller%20Object%20Reference) (DamageCauser :type Actor%20Object%20Reference))
  (Development|PrintString (Utilities|String|Append "Tomou dano" (Utilities|String|ToString(Float) Damage)) true true "(R=0.662500,G=0.076018,B=0.112948,A=1.000000)" 5.0))

(event Input|ActionEvents|InputActionDash
  (params (Key :type Key%20Structure :default "None")))

(event Input|ActionEvents|InputActionJump
  (params (Key :type Key%20Structure :default "None"))
  (:Pressed
    (Character|Jump)))

(event Input|ActionEvents|InputActionAtack
  (params (Key :type Key%20Structure :default "None"))
  (:Pressed
    (Class|PaperZDAnimInstance|JumptoNode (Variables|/Script/PaperZD.PaperZDAnimationComponent|GetAnimInstance (Variables|Default|GetAnimationComponent)) "Atack" "None")))

(event Input|AxisEvents|InputAxisRight
  (params (AxisValue :type Float%20%28single-precision%29))
  (if true
    (Pawn|Input|AddMovementInput "1.000000,0.000000,0.000000" AxisValue false)))

(fn ConstructionScript)

(fn SpawnDust
  (bind _sprite (Variables|Default|GetSprite))
  (bind _returnvalue (Transformation|GetWorldTransform _sprite))
  (Game|SpawnActorfromClass "/Game/Blueprints/Efects_Characters/BP_LandDust.BP_LandDust_C" (Math|Transform|MakeTransform (.location _returnvalue) (.rotation _returnvalue) "1.000000,1.000000,1.000000") "Undefined" 0 0))